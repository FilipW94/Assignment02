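; BP_IcePlatform is an ice platform that starts sinking at BeginPlay and destroys itself once it finishes.
; A Timeline sets the IcePlatform component's relative Z each update.
; Actor hits are filtered through BPI_Projectile to read the projectile's ammo type.
; Fire ammo destroys the platform immediately, while normal and ice ammo only print a no-effect debug message.
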(event Custom|OnActorHit_Event
  (params (SelfActor :type Actor%20Object%20Reference) (OtherActor :type Actor%20Object%20Reference) (NormalImpulse :type Vector) (Hit :type Hit%20Result%20Structure%20%28by%20ref%29))
  (if (Utilities|DoesObjectImplementInterface OtherActor "/Game/BPI_Projectile.BPI_Projectile_C")
    (bind _ammotypeoutput (Class|BPIProjectile|Projectile(Message) OtherActor))
    (switch Utilities|FlowControl|Switch|SwitchonE_AmmoSelection _ammotypeoutput
      (:NewEnumerator0
        (Development|PrintString "no offect" :!label _label))
      (:NewEnumerator1
        (Actor|DestroyActor))
      (:NewEnumerator2
        (goto _label)))))

(event EventBeginPlay
  (Utilities|FlowControl|Sequence
    (:then_0
      (EventDispatchers|BindEventtoOnActorHit (delegate Custom|OnActorHit_Event)))
    (:then_1
      (bind _icesinking (Timeline|Timeline Play)
        (:Update
          (Transformation|SetRelativeLocation (Variables|Default|GetIcePlatform) (Math|Vector|MakeVector 0.0 0.0 _icesinking) false false))
        (:Finished
          (Actor|DestroyActor))))))

(fn ConstructionScript)