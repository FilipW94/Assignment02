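; BP_DangerActor is a hazard actor that sends the player back to a start point instead of killing them.
; DeathFunction checks that the given actor is valid and is player character 0.
; It then teleports that character, without sweep, to the location of the PlayerStart the game mode finds by the name StartPosition.
; The event graph is empty, so the function relies on being called from elsewhere.
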(event EventBeginPlay)

(event EventTick
  (params (DeltaSeconds :type Float%20%28single-precision%29)))

(fn DeathFunction
  (params (PlayerACtor :type Actor%20Object%20Reference))
  (bind _returnvalue (Game|GetPlayerCharacter 0))
  (if (Utilities|IsValid PlayerACtor)
    (if (== PlayerACtor _returnvalue)
      (Transformation|SetActorLocation _returnvalue (.location (Transformation|GetActorTransform (Class|GameModeBase|FindPlayerStart (Game|GetGameMode) (Game|GetPlayerController 0) "StartPosition"))) false true)
      (return))))