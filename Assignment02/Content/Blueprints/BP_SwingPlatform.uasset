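; Swinging platform that pitches when a Normal Ammo projectile hits it, then swings back after a timed delay.
; Hits on SwingTarget are filtered through BI_Projectile and play the Swing timeline, which drives the target's relative pitch.
; When that finishes, a timer calls ResetSwing to reverse the same timeline.
; Tick shows the rounded countdown on two text renders, which return to the Timer value once the reversal completes.
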(event Custom|OnComponentHit_Event
  (params (HitComponent :type Primitive%20Component%20Object%20Reference) (OtherActor :type Actor%20Object%20Reference) (OtherComp :type Primitive%20Component%20Object%20Reference) (NormalImpulse :type Vector) (Hit :type Hit%20Result%20Structure%20%28by%20ref%29))
  (bind _timer (Variables|Default|GetTimer))
  (bind _returnvalue (Utilities|Text|ToText(Float) _timer "HalfToEven"))
  (if (Utilities|DoesObjectImplementInterface OtherActor "/Game/Blueprints/BI_Projectile.BI_Projectile_C")
    (bind _ammotypeoutput (Class|BIProjectile|Projectile(Message) OtherActor))
    (switch Utilities|FlowControl|Switch|SwitchonE_AmmoSelection _ammotypeoutput
      (:NewEnumerator0
        (Variables|Default|SetSwinginProgress true)
        (bind _swingfall (Timeline|Swing Play)
          (:Update
            (Transformation|SetRelativeRotation (Variables|Default|GetSwingTarget) (Math|Rotator|MakeRotator 0.0 _swingfall 0.0) false false))
          (:Finished
            (if (Variables|Default|GetSwinginProgress)
              (bind _returnvalue_2 (Utilities|Time|SetTimerbyEvent (delegate Custom|ResetSwing) _timer))
              (Variables|Default|SetTimerHandle _returnvalue_2)
              (else
                ;[1 1 1] Reset timer after is has gone back up
                (Rendering|Components|TextRender|SetText (Variables|Default|GetTextRender) _returnvalue)
                (Rendering|Components|TextRender|SetText (Variables|Default|GetTextRender1) _returnvalue)))))))))

(event Custom|ResetSwing
  (bind _timer (Variables|Default|GetTimer))
  (bind _returnvalue (Utilities|Text|ToText(Float) _timer "HalfToEven"))
  (Variables|Default|SetSwinginProgress false)
  (bind _swingfall (Timeline|Swing Reverse)
    (:Update
      (Transformation|SetRelativeRotation (Variables|Default|GetSwingTarget) (Math|Rotator|MakeRotator 0.0 _swingfall 0.0) false false))
    (:Finished
      (if (Variables|Default|GetSwinginProgress)
        (bind _returnvalue_2 (Utilities|Time|SetTimerbyEvent (delegate Custom|ResetSwing) _timer))
        (Variables|Default|SetTimerHandle _returnvalue_2)
        (else
          ;[1 1 1] Reset timer after is has gone back up
          (Rendering|Components|TextRender|SetText (Variables|Default|GetTextRender) _returnvalue)
          (Rendering|Components|TextRender|SetText (Variables|Default|GetTextRender1) _returnvalue))))))

(event EventBeginPlay
  (Collision|AssignOnComponentHit (Variables|Default|GetSwingTarget) (delegate Custom|OnComponentHit_Event)))

(event EventTick
  (params (DeltaSeconds :type Float%20%28single-precision%29))
  (bind _timerhandle (Variables|Default|GetTimerHandle))
  (bind _returnvalue (Utilities|Time|GetTimerRemainingTimebyHandle _timerhandle))
  (bind _returnvalue_2 (Math|Float|Round _returnvalue))
  (bind _returnvalue_3 (Utilities|Text|ToText(Integer) _returnvalue_2))
  ;[1 1 1] Countdown for swing
  (if (Class|KismetSystemLibrary|TimerExistsHandle _timerhandle)
    (Rendering|Components|TextRender|SetText (Variables|Default|GetTextRender) _returnvalue_3)
    (Rendering|Components|TextRender|SetText (Variables|Default|GetTextRender1) _returnvalue_3)))

(fn ConstructionScript)