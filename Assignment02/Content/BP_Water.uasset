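; BP_Water is a water actor that reacts to elemental projectiles hitting it.
; When its Cube component is overlapped by an actor implementing BPI_Projectile, it asks that actor for its ammo type via ProjectileMessage.
; Fire ammo spawns NS_Smoke and ice ammo spawns a BP_IcePlatform, both at the sweep result location, and either projectile is destroyed.
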(event OnComponentBeginOverlap(Cube)
  (params (OverlappedComponent :type Primitive%20Component%20Object%20Reference) (OtherActor :type Actor%20Object%20Reference) (OtherComp :type Primitive%20Component%20Object%20Reference) (OtherBodyIndex :type Integer) (bFromSweep :type Boolean) (SweepResult :type Hit%20Result%20Structure%20%28by%20ref%29))
  (if (Utilities|DoesObjectImplementInterface OtherActor "/Game/BPI_Projectile.BPI_Projectile_C")
    (bind _ammotypeoutput (Class|BPIProjectile|Projectile(Message) OtherActor))
    (switch Utilities|FlowControl|Switch|SwitchonE_AmmoSelection _ammotypeoutput
      (:NewEnumerator1
        (bind _output_get_location (|EmitterSpawnLocation SweepResult))
        (Niagara|SpawnSystematLocation "/Game/NS_Smoke.NS_Smoke" _output_get_location)
        (Actor|DestroyActor OtherActor))
      (:NewEnumerator2
        (bind _output_get_location_2 (|IcePlatformSpawnLocation SweepResult))
        (Actor|DestroyActor OtherActor)
        (Game|SpawnActorfromClass "/Game/BP_IcePlatform.BP_IcePlatform_C" (Math|Transform|MakeTransform _output_get_location_2 "0, 0, 0" "1.000000,1.000000,1.000000") "Undefined" "MultiplyWithRoot" 0 0)))))

(event EventBeginPlay)

(event Collision|EventActorBeginOverlap
  (params (OtherActor :type Actor%20Object%20Reference)))

(fn ConstructionScript)